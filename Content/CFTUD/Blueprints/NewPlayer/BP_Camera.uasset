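; BP_Camera drives camera control for its BP_Player owner, with free look and a lock-on toggle, and sets a starting control rotation on BeginPlay.
; Free look scales input by gamepad turn rate and delta time, applying pitch only when strictly inside YRange.
; While locked, look input is ignored and Tick aims control rotation from FollowCamera's relative location toward LockedEnemy.
; Tick also prints control rotation and draws a debug sphere on the locked enemy.
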(event `EnhancedInput|/Game/CFTUD/Blueprints/NewPlayer/Inputs/IA_Lock`
  (params (ActionValue :type Boolean) (ElapsedSeconds :type "Float (double-precision)") (TriggeredSeconds :type "Float (double-precision)") (InputAction :type "InputAction Object Reference" :default "/Game/CFTUD/Blueprints/NewPlayer/Inputs/IA_Lock.IA_Lock"))
  (bind _lock (`self.Lock`))
  (:`Triggered`
    (set `self.Lock` (not _lock))
    (if _lock
      _)))

(event `self.ReceiveTick`
  (params (DeltaSeconds :type "Float (single-precision)"))
  (bind _player (`self.Player`))
  (bind _returnvalue (`Pawn.GetController` _player))
  (bind _returnvalue_2 (`Actor.K2_GetActorLocation` (`self.LockedEnemy`)))
  (`KismetSystemLibrary.PrintString` (`KismetStringLibrary.Conv_RotatorToString` (`Controller.GetControlRotation` _returnvalue)) true true (struct :`G` 0.66 :`B` 1.0 :`A` 1.0) 0.0)
  (if (`self.Lock`)
    (`Controller.SetControlRotation` _returnvalue (`KismetMathLibrary.FindLookAtRotation` (`SceneComponent.RelativeLocation` (`/Game/CFTUD/Blueprints/NewPlayer/BP_Player.FollowCamera` _player)) _returnvalue_2))
    (`KismetSystemLibrary.DrawDebugSphere` _returnvalue_2 100.0 12 (struct :`R` 1.0 :`A` 1.0))))

(event `self.ReceiveBeginPlay`
  (bind _asbp_player (cast `/Game/CFTUD/Blueprints/NewPlayer/BP_Player` (`self.GetOwner`)))
  (set `self.Player` _asbp_player)
  (`Controller.SetControlRotation` (`Pawn.GetController` (`self.Player`)) (`KismetMathLibrary.MakeRotator` 0.0 350.0 90.0)))

(event `EnhancedInput|/Game/CFTUD/Blueprints/NewPlayer/Inputs/IA_Look`
  (params (ActionValue :type "Vector2D Structure") (ElapsedSeconds :type "Float (double-precision)") (TriggeredSeconds :type "Float (double-precision)") (InputAction :type "InputAction Object Reference" :default "/Game/CFTUD/Blueprints/NewPlayer/Inputs/IA_Look.IA_Look"))
  (bind _returnvalue (`GameplayStatics.GetWorldDeltaSeconds`))
  (bind (_axismultiply_x _axismultiply_y) (`KismetMathLibrary.BreakVector2D` (`self.AxisMultiply`)))
  (bind (_yrange_x _yrange_y) (`KismetMathLibrary.BreakVector2D` (`self.YRange`)))
  (bind (_yrange_x_2 _yrange_y_2) (`KismetMathLibrary.BreakVector2D` (`self.YRange`)))
  (bind _turnrategamepad (`self.TurnRateGamepad`))
  (bind _returnvalue_2 (`Pawn.GetController` (`self.Player`)))
  (bind (_returnvalue_roll _returnvalue_pitch _returnvalue_yaw) (`KismetMathLibrary.BreakRotator` (`Controller.GetControlRotation` _returnvalue_2)))
  (bind _returnvalue_3 (`KismetMathLibrary.FClamp` (+ _returnvalue_pitch (* (/ ActionValue_Y _axismultiply_y) _turnrategamepad _returnvalue)) _yrange_x _yrange_y))
  (:`Triggered`
    (if (not (`self.Lock`)) :!label _label
      (`Pawn.AddControllerYawInput` (`self.Player`) (* (* ActionValue_X _axismultiply_x) _turnrategamepad _returnvalue))
      (if (`KismetMathLibrary.InRange_FloatFloat` _returnvalue_3 _yrange_x_2 _yrange_y_2 false false)
        (`Controller.SetControlRotation` _returnvalue_2 (`KismetMathLibrary.MakeRotator` _returnvalue_roll _returnvalue_3 _returnvalue_yaw)))))
  (:`Completed`
    (goto _label)))