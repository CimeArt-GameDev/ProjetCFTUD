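; Player attack component that runs a three-hit melee montage combo from the IA_Attack input.
; An attack starts when not blocking or already attacking, locks rotation and plays the montage for the current count, with later hits starting partway in.
; Otherwise the press is buffered in SaveAttack, which the ComboAttack event consumes to chain the next hit.
; ResetCombo clears the count, buffer and attacking flag.
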(event `self.ReceiveBeginPlay`
  (bind _asbp_player (cast `/Game/CFTUD/Blueprints/NewPlayer/BP_Player` (`self.GetOwner`)))
  (set `self.Mesh` (`Character.Mesh` _asbp_player)))

(event `EnhancedInput|/Game/CFTUD/Blueprints/NewPlayer/Inputs/IA_Attack`
  (params (ActionValue :type Boolean) (ElapsedSeconds :type "Float (double-precision)") (TriggeredSeconds :type "Float (double-precision)") (InputAction :type "InputAction Object Reference" :default "/Game/CFTUD/Blueprints/NewPlayer/Inputs/IA_Attack.IA_Attack"))
  (:`Started`
    (if (and (not (`|GetInputActionValue`)) (not (`self.IsAttacking?`)))
      (set `self.IsAttacking?` true)
      (set `self.CanRotate?` false)
      (switch `int` (`self.AttackCount`) :!label _label
        (:`0`
          (set `self.AttackCount` 1)
          (`|PlayMontage` null "/Game/CFTUD/Blueprints/NewPlayer/Animations/Fight/FirstSlashMontage.FirstSlashMontage"))
        (:`1`
          (set `self.AttackCount` 2)
          (`|PlayMontage` null "/Game/CFTUD/Blueprints/NewPlayer/Animations/Fight/SecondSlashMontage.SecondSlashMontage" 1.0 0.67))
        (:`2`
          (`|PlayMontage` null "/Game/CFTUD/Blueprints/NewPlayer/Animations/Fight/LastAttackComboMontage.LastAttackComboMontage" 1.0 1.33)))
      (else
        (set `self.SaveAttack` true)))))

(event `ComboAttack`
  (if (`self.SaveAttack`)
    (set `self.SaveAttack` false)
    (goto _label)))

(event `ResetCombo`
  (set `self.AttackCount` 0)
  (set `self.SaveAttack` false)
  (set `self.IsAttacking?` false))