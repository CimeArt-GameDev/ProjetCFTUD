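; Player character with Enhanced Input movement, dash, block, aim, interaction and a work-in-progress lock-on.
; Dash precomputes a ground-following path with forward and downward line traces, then replays a timeline over each segment before cooldown.
; Block drives camera-boom timelines, with aim adding a crosshair and camera-aligned rotation.
; Overlap spheres feed interaction and nearest-enemy selection; attack input and lock-on camera code are disconnected, leaving a montage combo event.
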(event `self.ReceiveBeginPlay`
  ;[1 0 0] Begin Play
  (`EnhancedInputSubsystemInterface.AddMappingContext` (pcsubsystem `EnhancedInputLocalPlayerSubsystem` (`GameplayStatics.GetPlayerController` 0)) "/Game/CFTUD/Blueprints/NewPlayer/Inputs/IMC_Player.IMC_Player" 0 (struct))
  (bind _asabp_player (cast `/Game/CFTUD/Blueprints/NewPlayer/ABP_Player` (`SkeletalMeshComponent.GetAnimInstance` (`self.Mesh`))))
  (set `self.AnimInstanceRef` _asabp_player))

(event `EnhancedInput|/Game/CFTUD/Blueprints/NewPlayer/Inputs/IA_Look`
  (params (ActionValue :type "Vector2D Structure") (ElapsedSeconds :type "Float (double-precision)") (TriggeredSeconds :type "Float (double-precision)") (InputAction :type "InputAction Object Reference" :default "/Game/CFTUD/Blueprints/NewPlayer/Inputs/IA_Look.IA_Look"))
  ;[1 1 1] Look and movements
)

(event `EnhancedInput|/Game/CFTUD/Blueprints/NewPlayer/Inputs/IA_Move`
  (params (ActionValue :type "Vector2D Structure") (ElapsedSeconds :type "Float (double-precision)") (TriggeredSeconds :type "Float (double-precision)") (InputAction :type "InputAction Object Reference" :default "/Game/CFTUD/Blueprints/NewPlayer/Inputs/IA_Move.IA_Move"))
  (bind (_returnvalue_x _returnvalue_y) (`KismetMathLibrary.BreakVector2D` (`|GetInputActionValue`)))
  (bind (_returnvalue_roll _returnvalue_pitch _returnvalue_yaw) (`KismetMathLibrary.BreakRotator` (`SpringArmComponent.GetTargetRotation` (`self.CameraBoom`))))
  (bind (_returnvalue_roll_2 _returnvalue_pitch_2 _returnvalue_yaw_2) (`KismetMathLibrary.BreakRotator` (`KismetMathLibrary.Conv_VectorToRotator` (`KismetMathLibrary.MakeVector` (* _returnvalue_y -1.0) (* _returnvalue_x -1.0)))))
  ;[1 1 1] Look and movements
  (:`Triggered`
    (if (and (not (`self.GetBlockInput`)) (`self.CanRotate?`)) :!label _label
      (`self.K2_SetActorRotation` (`KismetMathLibrary.RInterpTo` (`self.K2_GetActorRotation`) (`KismetMathLibrary.MakeRotator` 0.0 0.0 (+ (- _returnvalue_yaw 90.0) _returnvalue_yaw_2)) (`GameplayStatics.GetWorldDeltaSeconds`) 4.0))))
  (:`Completed`
    (goto _label)))

(event `EnhancedInput|/Game/CFTUD/Blueprints/NewPlayer/Inputs/IA_Dash`
  (params (ActionValue :type Boolean) (ElapsedSeconds :type "Float (double-precision)") (TriggeredSeconds :type "Float (double-precision)") (InputAction :type "InputAction Object Reference" :default "/Game/CFTUD/Blueprints/NewPlayer/Inputs/IA_Dash.IA_Dash"))
  (bind (_returnvalue_x _returnvalue_y) (`KismetMathLibrary.BreakVector2D` (`self.GetMovementInputs`)))
  (bind _capsulecomponent (`self.CapsuleComponent`))
  (bind _index (`self.Index`))
  (bind _index_2 (`self.Index`))
  ;[1 1 1] Dash (A refaire : voir dash system Zelda BOTW)
  (:`Started`
    (if (not (`self.DashOnCooldown`))
      (set `self.Index` 0)
      (bind _curve (`self.DashCurve` true (`KismetMathLibrary.SelectInt` 5 7 (`self.GetBlockInput`)) (`KismetMathLibrary.SelectVector` (`SceneComponent.GetForwardVector` _capsulecomponent) (* (`SceneComponent.GetRightVector` _capsulecomponent) (`KismetMathLibrary.SelectFloat` 1.0 -1.0 (> _returnvalue_y 0.0))) (not (`self.GetBlockInput`)))))
      (bind (_direction _distance) (`Timeline|Dash Timeline` :!label _label_2)
        (:`Update`
          (`self.K2_SetActorLocation` (`KismetMathLibrary.VLerp` (`|GetArrayItem` _curve _index) (`|GetArrayItem` _curve (+ _index 1)) _distance))
          (`ActorComponent.SetActive` (`self.Niagara`) true true))
        (:`Finished`
          (if (< _index_2 (- (`KismetArrayLibrary.Array_LastIndex` _curve) 1))
            (`/Engine/EditorBlueprintResources/StandardMacros.IncrementInt` _index_2
              (:`  `
                (goto _label_2 :!via `PlayFromStart`)))
            (else
              (set `self.DashOnCooldown` true)
              (`KismetSystemLibrary.K2_SetTimerDelegate` (delegate `ResetDashCooldown`) (`self.DashCooldown`))
              (goto _label_2 :!via `SetNewTime`))))))))

(event `ResetDashCooldown`
  ;[1 1 1] Dash (A refaire : voir dash system Zelda BOTW)
  (set `self.DashOnCooldown` false))

(event `EnhancedInput|/Game/CFTUD/Blueprints/NewPlayer/Inputs/IA_Block`
  (params (ActionValue :type Boolean) (ElapsedSeconds :type "Float (double-precision)") (TriggeredSeconds :type "Float (double-precision)") (InputAction :type "InputAction Object Reference" :default "/Game/CFTUD/Blueprints/NewPlayer/Inputs/IA_Block.IA_Block"))
  (bind (_returnvalue_x _returnvalue_y) (`KismetMathLibrary.BreakVector2D` (`self.GetMovementInputs`)))
  (bind _crosshairwidgetref (`self.CrosshairWidgetRef`))
  (bind (_returnvalue_roll _returnvalue_pitch _returnvalue_yaw) (`KismetMathLibrary.BreakRotator` (`SpringArmComponent.GetTargetRotation` (`self.CameraBoom`))))
  ;[1 1 1] Block
  (:`Triggered`
    ;;[1 1 1] Feeling pas ouf revoir ref dark souls shield, lords of the fallen
    (`|ExecutionSequence`
      (:`then_0`
        (if (or (!= _returnvalue_x 0.0) (!= _returnvalue_y 0.0))
          (`SceneComponent.K2_SetWorldRotation` (`self.CapsuleComponent`) (`KismetMathLibrary.RLerp` (`KismetMathLibrary.Conv_VectorToRotator` (`self.GetActorForwardVector`)) (`KismetMathLibrary.MakeRotator` 0.0 0.0 _returnvalue_yaw) 0.1 true) false false)
          (`self.PlayAnimMontage` "/Game/CFTUD/Blueprints/NewPlayer/Animations/Fight/BlockLoop_Montage.BlockLoop_Montage")))
      (:`then_1`
        ;;[1 1 1] Aim system pas prioritaire
        (if (and (`|GetInputActionValue`) (`|GetInputActionValue`)) :!label _label_3
          (`self.ResetCombo`)
          (set `self.CanRotate?` true)
          (`self.RotatePlayerWithCameraView`)
          (`/Engine/EditorBlueprintResources/StandardMacros.DoOnce` false :!label _label_4
            (:`Completed`
              (bind _returnvalue (`|CreateWidget` "/Game/CFTUD/Blueprints/NewPlayer/WBP_Crosshair.WBP_Crosshair_C"))
              (bind _output_get (set `self.CrosshairWidgetRef` _returnvalue))
              (`UserWidget.AddToViewport` _output_get 0)
              (bind (_direction _location) (`Timeline|ChangeSpringArmLocation` :!label _label_5)
                (:`Update`
                  (`SceneComponent.K2_SetRelativeLocation` (`self.CameraBoom`) _location false false)))))
          (else
            (`/Engine/EditorBlueprintResources/StandardMacros.IsValid` _crosshairwidgetref
              (:`Is Valid`
                (`/Game/CFTUD/Blueprints/NewPlayer/WBP_Crosshair.Erase Widget` _crosshairwidgetref)
                (set `self.CrosshairWidgetRef` null)
                (set `self.CanRotate?` false)
                (`|ExecutionSequence`
                  (:`then_0`
                    (goto _label_4 :!via `Reset`))
                  (:`then_1`
                    (goto _label_5 :!via `Reverse`))))))))))
  (:`Started`
    (bind (_direction_2 _length) (`Timeline|SetArmLength` :!label _label_6)
      (:`Update`
        ;;[1 1 1] Jouer aussi sur le FOV de la cam
        (set `SpringArmComponent.TargetArmLength` (* _length 100.0) (`self.CameraBoom`)))))
  (:`Completed`
    (`|ExecutionSequence`
      (:`then_0`
        (goto _label_6 :!via `Reverse`))
      (:`then_1`
        (`self.StopAnimMontage` "/Game/CFTUD/Blueprints/NewPlayer/Animations/Fight/BlockLoop_Montage.BlockLoop_Montage")
        (goto _label_3)))))

(event `EnhancedInput|/Game/CFTUD/Blueprints/NewPlayer/Inputs/IA_Attack`
  (params (ActionValue :type Boolean) (ElapsedSeconds :type "Float (double-precision)") (TriggeredSeconds :type "Float (double-precision)") (InputAction :type "InputAction Object Reference" :default "/Game/CFTUD/Blueprints/NewPlayer/Inputs/IA_Attack.IA_Attack"))
  ;[1 1 1] Attack Bug en meme temps que le aim
)

(event `ComboAttack`
  (bind (_returnvalue_x _returnvalue_y) (`KismetMathLibrary.BreakVector2D` (`self.GetMovementInputs`)))
  (bind _mesh (`self.Mesh`))
  (bind (_returnvalue_roll _returnvalue_pitch _returnvalue_yaw) (`KismetMathLibrary.BreakRotator` (`KismetMathLibrary.Conv_VectorToRotator` (`SceneComponent.GetForwardVector` (`self.FollowCamera`)))))
  (bind (_returnvalue_roll_2 _returnvalue_pitch_2 _returnvalue_yaw_2) (`KismetMathLibrary.BreakRotator` (`KismetMathLibrary.Conv_VectorToRotator` (`KismetMathLibrary.MakeVector` (* _returnvalue_x -1.0) _returnvalue_y))))
  ;[1 1 1] Attack Bug en meme temps que le aim
  (if (`self.SaveAttack`)
    (set `self.SaveAttack` false)
    (switch `int` (`self.AttackCount`)
      (:`0`
        (set `self.AttackCount` 1)
        (`|PlayMontage` _mesh "/Game/CFTUD/Blueprints/NewPlayer/Animations/Fight/FirstSlashMontage.FirstSlashMontage"
          (:`then`
            (set `self.Rotaaaaaaaaaaaaaaaate` true :!label _label_7)
            (`SceneComponent.K2_SetWorldRotation` (`self.CapsuleComponent`) (`KismetMathLibrary.MakeRotator` 0.0 0.0 (+ _returnvalue_yaw _returnvalue_yaw_2)) false false))
          (:`OnCompleted`
            (set `self.Rotaaaaaaaaaaaaaaaate` false :!label _label_8))))
      (:`1`
        (set `self.AttackCount` 2)
        (`|PlayMontage` _mesh "/Game/CFTUD/Blueprints/NewPlayer/Animations/Fight/SecondSlashMontage.SecondSlashMontage" 1.0 0.67
          (:`then`
            (goto _label_7))
          (:`OnCompleted`
            (goto _label_8))))
      (:`2`
        (`|PlayMontage` _mesh "/Game/CFTUD/Blueprints/NewPlayer/Animations/Fight/LastAttackComboMontage.LastAttackComboMontage" 1.0 1.33
          (:`then`
            (goto _label_7))
          (:`OnCompleted`
            (goto _label_8)))))))

(event `ResetCombo`
  ;[1 1 1] Attack Bug en meme temps que le aim
  (set `self.AttackCount` 0)
  (set `self.SaveAttack` false)
  (set `self.IsAttacking?` false))

(event `self.Interaction Sphere.OnComponentBeginOverlap`
  (params (OverlappedComponent :type "PrimitiveComponent Object Reference") (OtherActor :type "Actor Object Reference") (OtherComp :type "PrimitiveComponent Object Reference") (OtherBodyIndex :type Integer) (bFromSweep :type Boolean) (SweepResult :type "HitResult Structure (by ref)"))
  ;[1 1 1] Interaction
  (if (`KismetSystemLibrary.DoesImplementInterface` OtherActor "/Game/CFTUD/Blueprints/BPI_Interact.BPI_Interact_C")
    (bind _asbp_interactible (cast `/Game/CFTUD/Blueprints/Object/Interractible/BP_Interactible` OtherActor))
    (set `self.Interactible` _asbp_interactible)))

(event `self.Interaction Sphere.OnComponentEndOverlap`
  (params (OverlappedComponent :type "PrimitiveComponent Object Reference") (OtherActor :type "Actor Object Reference") (OtherComp :type "PrimitiveComponent Object Reference") (OtherBodyIndex :type Integer))
  ;[1 1 1] Interaction
  (set `self.Interactible` null))

(event `EnhancedInput|/Game/CFTUD/Blueprints/NewPlayer/Inputs/IA_Interact`
  (params (ActionValue :type Boolean) (ElapsedSeconds :type "Float (double-precision)") (TriggeredSeconds :type "Float (double-precision)") (InputAction :type "InputAction Object Reference" :default "/Game/CFTUD/Blueprints/NewPlayer/Inputs/IA_Interact.IA_Interact"))
  (bind _interactible (`self.Interactible`))
  ;[1 1 1] Interaction
  (:`Started`
    (`/Engine/EditorBlueprintResources/StandardMacros.IsValid` _interactible
      (:`Is Valid`
        (`KismetSystemLibrary.PrintString` (select `/Game/CFTUD/Blueprints/Object/Interractible/Enum_Interactible` (`/Game/CFTUD/Blueprints/Object/Interractible/BP_Interactible.Type` _interactible) :`NewEnumerator0` "Opening Chest" :`NewEnumerator1` "Pull Lever" :`NewEnumerator2` "Push Button"))
        (`|PlayMontage` (`self.Mesh`)
          (:`OnCompleted`
            (`/Game/CFTUD/Blueprints/BPI_Interact.Interract` (`self.Interactible`))))))))

(event `self.LockRange.OnComponentBeginOverlap`
  (params (OverlappedComponent :type "PrimitiveComponent Object Reference") (OtherActor :type "Actor Object Reference") (OtherComp :type "PrimitiveComponent Object Reference") (OtherBodyIndex :type Integer) (bFromSweep :type Boolean) (SweepResult :type "HitResult Structure (by ref)"))
  ;[1 1 1] Lock
  ;;[0 0.1331 1] Va être refait ! Ne pas prendre en compte
  (bind _ascharacter (cast `Character` OtherActor))
  (cast `/Game/CFTUD/Blueprints/NewPlayer/BP_Player` _ascharacter
    (:`CastFailed`
      (`KismetArrayLibrary.Array_AddUnique` (`self.EnemiesInLockRange`) _ascharacter)
      (`KismetSystemLibrary.PrintString` "Hello"))))

(event `self.LockRange.OnComponentEndOverlap`
  (params (OverlappedComponent :type "PrimitiveComponent Object Reference") (OtherActor :type "Actor Object Reference") (OtherComp :type "PrimitiveComponent Object Reference") (OtherBodyIndex :type Integer))
  ;[1 1 1] Lock
  ;;[0 0.1331 1] Va être refait ! Ne pas prendre en compte
  (bind _ascharacter (cast `Character` OtherActor))
  (`KismetArrayLibrary.Array_RemoveItem` (`self.EnemiesInLockRange`) _ascharacter)
  (set `self.Locked?` false))

(event `EnhancedInput|/Game/CFTUD/Blueprints/NewPlayer/Inputs/IA_Lock`
  (params (ActionValue :type Boolean) (ElapsedSeconds :type "Float (double-precision)") (TriggeredSeconds :type "Float (double-precision)") (InputAction :type "InputAction Object Reference" :default "/Game/CFTUD/Blueprints/NewPlayer/Inputs/IA_Lock.IA_Lock"))
  (bind _returnvalue (`self.K2_GetActorLocation`))
  ;[1 1 1] Lock
  ;;[0 0.1331 1] Va être refait ! Ne pas prendre en compte
  (:`Started`
    (if (and (`KismetArrayLibrary.Array_IsNotEmpty` (`self.EnemiesInLockRange`)) (not (`self.Locked?`)))
      (for _array_element (`self.EnemiesInLockRange`)
        (`/Engine/EditorBlueprintResources/StandardMacros.IsValid` (`self.ClosestEnemy`)
          (:`Is Valid`
            (if (< (`KismetMathLibrary.Vector_Distance` (`self.K2_GetActorLocation` _array_element) _returnvalue) (`KismetMathLibrary.Vector_Distance` _returnvalue (`self.K2_GetActorLocation` (`self.ClosestEnemy`))))
              (set `self.ClosestEnemy` _array_element)))
          (:`Is Not Valid`
            (set `self.ClosestEnemy` _array_element))))
      (`/Engine/EditorBlueprintResources/StandardMacros.IsValid` (`self.ClosestEnemy`)
        (:`Is Valid`
          (set `self.Locked?` true)))
      (else
        (set `self.Locked?` false)))))

(event `self.ReceiveTick`
  (params (DeltaSeconds :type "Float (single-precision)"))
  ;[1 1 1] Lock
  ;;[0 0.1331 1] Va être refait ! Ne pas prendre en compte
  ;;;[1 1 1] A revoir avec des ref
  ;;;;[1 0 0] On Tick
)

(event `Key|NumPadOne`
  (params (Key :type "Key Structure"))
  ;[1 1 1] Lock
  ;;[1 0.7543 0] Juste pour du test
  (:`Pressed`
    (bind _returnvalue (`GameplayStatics.GetActorOfClass` "/Game/CFTUD/Blueprints/Enemy/Boss1-VCamille/BP_Boss1Camille.BP_Boss1Camille_C"))
    (bind _isa (`/Engine/EditorBlueprintResources/StandardMacros.FlipFlop`)
      (:`A`
        _)
      (:`B`
        _))
    (`/Game/CFTUD/Blueprints/Enemy/Boss1-VCamille/BP_Boss1Camille.DebugSetStage` _returnvalue _isa)))

(event `Key|NumPadTwo`
  (params (Key :type "Key Structure"))
  ;[1 1 1] Lock
  ;;[1 0.7543 0] Juste pour du test
  (:`Pressed`
    (bind _returnvalue (`GameplayStatics.GetActorOfClass` "/Game/CFTUD/Blueprints/Player2/BP_Player2.BP_Player2_C"))
    (`Controller.Possess` (`GameplayStatics.GetPlayerController` 0) _returnvalue)))

(fn `DashCurve`
  (params (`Debug?` :type Boolean) (Multiplier :type Integer) (Direction :type "Vector Structure"))
  (returns (Curve :type "Array of Vector Structure"))
  (locals (`Pick A` :type Boolean :default true) (LocationArray :type "Array of Vector Structure") (`Show Debug` :type Boolean))
  (bind _locationarray (`local.LocationArray`))
  (bind _locationarray_2 (`local.LocationArray`))
  (bind _returnvalue (`KismetMathLibrary.SelectVector` (`self.K2_GetActorLocation`) (`self.New Transform`) (`local.Pick A`)))
  (set `local.Show Debug` `Debug?`)
  (`KismetArrayLibrary.Array_Clear` (`local.LocationArray`))
  (`KismetArrayLibrary.Array_Add` (`local.LocationArray`) (`self.K2_GetActorLocation`))
  (for _ (range (+ Multiplier 1))
    (bind (_outhit _returnvalue_2) (`KismetSystemLibrary.LineTraceSingle` :`Start` _returnvalue :`End` (+ _returnvalue (* Direction 100.0)) :`TraceChannel` "TraceTypeQuery1" :`DrawDebugType` (select `bool` (`local.Show Debug`) :`true` "Persistent" :!type "EDrawDebugTrace Enum")))
    (if _returnvalue_2
      (break)
      (else
        (set `local.Pick A` false)
        (bind (_outhit_2 _returnvalue_3) (`KismetSystemLibrary.LineTraceSingle` :`Start` (`.TraceEnd` (`GameplayStatics.BreakHitResult` _outhit)) :`End` (`KismetMathLibrary.MakeVector` (.x (`.TraceEnd` (`GameplayStatics.BreakHitResult` _outhit))) (.y (`.TraceEnd` (`GameplayStatics.BreakHitResult` _outhit))) (- (.z (`.TraceEnd` (`GameplayStatics.BreakHitResult` _outhit))) 250.0)) :`TraceChannel` "TraceTypeQuery1" :`DrawDebugType` (select `bool` (`local.Show Debug`) :`true` "Persistent" :!type "EDrawDebugTrace Enum") :`TraceColor` (struct :`G` 1.0 :`A` 1.0)))
        (if _returnvalue_3
          (bind _output_get (set `self.New Transform` (`KismetMathLibrary.MakeVector` (.x (`.TraceStart` (`GameplayStatics.BreakHitResult` _outhit_2))) (.y (`.TraceStart` (`GameplayStatics.BreakHitResult` _outhit_2))) (+ (.z (`.Location` (`GameplayStatics.BreakHitResult` _outhit_2))) 90.0))))
          (`KismetArrayLibrary.Array_Add` _locationarray_2 _output_get)
          (else
            (bind _output_get_2 (set `self.New Transform` (`KismetMathLibrary.MakeVector` (.x (`.TraceStart` (`GameplayStatics.BreakHitResult` _outhit_2))) (.y (`.TraceStart` (`GameplayStatics.BreakHitResult` _outhit_2))) (.z (`.TraceStart` (`GameplayStatics.BreakHitResult` _outhit_2))))))
            (`KismetArrayLibrary.Array_Add` _locationarray_2 _output_get_2))))))
  (set `local.Pick A` true)
  (if (`local.Show Debug`)
    (for (_array_element _array_index) _locationarray
      (if (< _array_index (`KismetArrayLibrary.Array_LastIndex` _locationarray))
        (`KismetSystemLibrary.DrawDebugLine` _array_element (`|GetArrayItem` _locationarray (+ _array_index 1)) (struct :`G` 0.197002 :`B` 1.0 :`A` 1.0) 100.0 5.0))))
  (return (`local.LocationArray`)))

(fn `GetAttackInput`
  (returns (ReturnValue :type Boolean))
  (return (`|GetInputActionValue`)))

(fn `GetBlockInput`
  (returns (`IsBlocking?` :type Boolean))
  (return (`|GetInputActionValue`)))

(fn `GetDashInput`
  (returns (ReturnValue :type Boolean))
  (return (`|GetInputActionValue`)))

(fn `GetDodgeInput`
  (returns (`IsDodging?` :type Boolean))
  (return (`|GetInputActionValue`)))

(fn `GetMovementInputs`
  (returns (ReturnValue :type "Vector2D Structure"))
  (return (`|GetInputActionValue`)))

(fn `RotateCameraWithPlayerRotation`
  (bind (_returnvalue_x _returnvalue_y) (`KismetMathLibrary.BreakVector` (`self.GetVelocity`)))
  (bind (_returnvalue_x_2 _returnvalue_y_2) (`KismetMathLibrary.BreakVector2D` (`self.GetMovementInputs`)))
  (bind _yinput (`self.yInput`))
  (bind (_returnvalue_x_3 _returnvalue_y_3) (`KismetMathLibrary.BreakVector` (`KismetMathLibrary.Normal` (`KismetMathLibrary.MakeVector` _returnvalue_x_2 _returnvalue_y_2))))
  (bind _output_get (set `self.yInput` _returnvalue_y_3))
  (if (!= _output_get 0.0)
    (`self.AddControllerYawInput` (* (* _yinput (`KismetMathLibrary.MultiplyMultiply_FloatFloat` (`KismetMathLibrary.Abs` _yinput) (`self.camAngleExponent`))) 100.0 (/ (`KismetMathLibrary.VSize` (`KismetMathLibrary.MakeVector` _returnvalue_x _returnvalue_y)) 379.0) (`self.camRotationFactor`) (`GameplayStatics.GetWorldDeltaSeconds`)))))

(fn `RotatePlayerWithCameraView`
  (locals (AdditiveRotation :type "Float (double-precision)"))
  (bind (_returnvalue_x _returnvalue_y) (`KismetMathLibrary.BreakVector2D` (`self.GetMovementInputs`)))
  (bind _capsulecomponent (`self.CapsuleComponent`))
  (bind (_returnvalue_roll _returnvalue_pitch _returnvalue_yaw) (`KismetMathLibrary.BreakRotator` (`SpringArmComponent.GetTargetRotation` (`self.CameraBoom`))))
  (bind (_returnvalue_roll_2 _returnvalue_pitch_2 _returnvalue_yaw_2) (`KismetMathLibrary.BreakRotator` (`KismetMathLibrary.Conv_VectorToRotator` (`KismetMathLibrary.MakeVector` (* _returnvalue_x -1.0) _returnvalue_y))))
  (if (and (`self.CanRotate?`) (not (`|GetInputActionValue`)))
    (if (not (`|GetInputActionValue`))
      (if (`self.IsAttacking?`)
        (set `local.AdditiveRotation` _returnvalue_yaw_2)
        (`SceneComponent.K2_SetWorldRotation` _capsulecomponent (`KismetMathLibrary.RLerp` (`KismetMathLibrary.Conv_VectorToRotator` (`self.GetActorForwardVector`)) (`KismetMathLibrary.MakeRotator` 0.0 0.0 (`local.AdditiveRotation`)) (* (`GameplayStatics.GetWorldDeltaSeconds`) 2.0)) false false)
        (else
          (set `local.AdditiveRotation` _returnvalue_yaw_2)
          (`SceneComponent.K2_SetWorldRotation` _capsulecomponent (`KismetMathLibrary.MakeRotator` 0.0 0.0 (+ (`local.AdditiveRotation`) _returnvalue_yaw)) false false :!label _label)))
      (else
        (set `local.AdditiveRotation` 0.0)
        (goto _label)))))

(fn `UserConstructionScript`)