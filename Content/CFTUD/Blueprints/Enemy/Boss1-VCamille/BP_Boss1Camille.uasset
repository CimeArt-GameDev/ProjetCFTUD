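; BP_Boss1Camille is the Blueprint for the Camille boss enemy, tracking its health and fight stage.
; AnyDamage subtracts from CurrentHealth and raises Stage once health drops below zero while Stage is under 1, although its comment describes a 50% threshold.
; DebugSetStage forces stage 0 or 1, prints it, then has the AIC_Boss1Camille controller run the BT_Boss1Camille behavior tree.
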(event `self.ReceiveAnyDamage`
  (params (Damage :type "Float (single-precision)") (DamageType :type "DamageType Object Reference") (InstigatedBy :type "Controller Object Reference") (DamageCauser :type "Actor Object Reference"))
  ;[1 1 1] Take Damage
  (bind _output_get (set `self.CurrentHealth` (- (`self.CurrentHealth`) Damage)))
  ;[1 1 1] If Boss HP < 50% , get in stage 1
  (if (and (< _output_get 0.0) (< (`self.Stage`) 1))
    (`/Engine/EditorBlueprintResources/StandardMacros.IncrementInt` (`self.Stage`))))

(event `DebugSetStage`
  (params (FinalStage :type Boolean))
  (bind _output_get (set `self.Stage` (`KismetMathLibrary.SelectInt` 1 0 FinalStage)))
  (`KismetSystemLibrary.PrintString` (`KismetStringLibrary.Concat_StrStr` "Boss1Cam Stage : " (`KismetStringLibrary.Conv_IntToString` _output_get)))
  (bind _asaic_boss_1camille (cast `/Game/CFTUD/Blueprints/Enemy/Boss1-VCamille/AIC_Boss1Camille` (`self.GetController`)))
  (`AIController.RunBehaviorTree` _asaic_boss_1camille "/Game/CFTUD/Blueprints/Enemy/Boss1-VCamille/BT_Boss1Camille.BT_Boss1Camille"))

(fn `UserConstructionScript`)