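; BP_Enemy is an enemy Blueprint, apparently a sentinel, with an entrance animation and a mostly unwired chase behavior.
; BeginPlay caches the ThirdPersonCharacter as Player, and the ActivateSentinel event plays the AM_Entrance montage on the mesh.
; The AI perception update event is empty.
; Disconnected nodes hold an AIMoveTo chase toward the player with a debug print, plus an unused ActivateSentinel call.
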(event `self.ReceiveBeginPlay`
  (bind _returnvalue (`GameplayStatics.GetActorOfClass` "/Game/Import/ThirdPersonCPP/Blueprints/ThirdPersonCharacter.ThirdPersonCharacter_C"))
  (set `self.Player` _returnvalue))

(event `ActivateSentinel`
  (`|PlayMontage` (`self.Mesh`) "/Game/CFTUD/OLD/OldPlayers/Animations/AnimationSequences/Entrance/AM_Entrance.AM_Entrance"))

(event `self.AIPerception.OnTargetPerceptionUpdated`
  (params (Actor :type "Actor Object Reference") (Stimulus :type "AIStimulus Structure")))

(fn `UserConstructionScript`)