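; BP_Boss1 is the first boss enemy, a Sentinel with an entrance animation.
; On BeginPlay it finds the BP_CharacterTest_Child actor and stores it as the Player reference.
; Its ActivateSentinel event plays the AM_Entrance montage on the mesh.
; The AI perception and Tick events are empty, and leftover cast and AI move-to nodes are disconnected, so it has no active chase behavior.
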(event `self.AIPerception.OnTargetPerceptionUpdated`
  (params (Actor :type "Actor Object Reference") (Stimulus :type "AIStimulus Structure"))
  ;[1 1 1] Comment
)

(event `self.ReceiveBeginPlay`
  (bind _returnvalue (`GameplayStatics.GetActorOfClass` "/Game/CFTUD/Blueprints/Player/BP_CharacterTest_Child.BP_CharacterTest_Child_C"))
  (set `self.Player` _returnvalue))

(event `ActivateSentinel`
  (`|PlayMontage` (`self.Mesh`) "/Game/CFTUD/Characters/Animations/AnimationSequences/Entrance/AM_Entrance.AM_Entrance"))

(event `self.ReceiveTick`
  (params (DeltaSeconds :type "Float (single-precision)")))

(fn `UserConstructionScript`)