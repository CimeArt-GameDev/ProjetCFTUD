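; Player Blueprint that handles Enhanced Input actions and shows their state as on-screen debug text.
; BeginPlay adds the player mapping context; attack, block, dodge and interact play montages, while other actions toggle combat/exploration mode and sprinting.
; GetAllInputValue gathers input values and state, which Tick prints each frame before overwriting Sprinting with a velocity check.
; Any key press records whether a keyboard is in use.
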(event `Key|AnyKey`
  (params (Key :type "Key Structure"))
  (:`Pressed`
    (set `self.IsKeyboardUsed` (`KismetInputLibrary.Key_IsKeyboardKey` Key))))

(event `self.ReceiveBeginPlay`
  (`EnhancedInputSubsystemInterface.AddMappingContext` (pcsubsystem `EnhancedInputLocalPlayerSubsystem` (`GameplayStatics.GetPlayerController` 0)) "/Game/CFTUD/Blueprints/Player/Input/IMC_Player.IMC_Player" 0))

(event `self.ReceiveTick`
  (params (DeltaSeconds :type "Float (single-precision)"))
  (`KismetSystemLibrary.PrintString` (`KismetStringLibrary.Concat_StrStr` "Jumping : " (`KismetStringLibrary.Conv_BoolToString` (`.IsJumping` (`self.GetAllInputValue`)))) true true (struct :`G` 0.66 :`B` 1.0 :`A` 1.0) 0.0)
  (`KismetSystemLibrary.PrintString` (`KismetStringLibrary.Concat_StrStr` "Sprinting : " (`KismetStringLibrary.Conv_BoolToString` (`.IsSprinting` (`self.GetAllInputValue`)))) true true (struct :`G` 0.66 :`B` 1.0 :`A` 1.0) 0.0)
  (`KismetSystemLibrary.PrintString` (`KismetStringLibrary.Concat_StrStr` "Playing Mode : " (`.PlayingMode` (`self.GetAllInputValue`))) true true (struct :`G` 0.66 :`B` 1.0 :`A` 1.0) 0.0)
  (`KismetSystemLibrary.PrintString` (`KismetStringLibrary.Concat_StrStr` "Interacting : " (`KismetStringLibrary.Conv_BoolToString` (`.IsInteracting` (`self.GetAllInputValue`)))) true true (struct :`G` 0.66 :`B` 1.0 :`A` 1.0) 0.0)
  (`KismetSystemLibrary.PrintString` (`KismetStringLibrary.Concat_StrStr` "Dodging : " (`KismetStringLibrary.Conv_BoolToString` (`.IsDodging` (`self.GetAllInputValue`)))) true true (struct :`G` 0.66 :`B` 1.0 :`A` 1.0) 0.0)
  (`KismetSystemLibrary.PrintString` (`KismetStringLibrary.Concat_StrStr` "Blocking : " (`KismetStringLibrary.Conv_BoolToString` (`.IsBlocking` (`self.GetAllInputValue`)))) true true (struct :`G` 0.66 :`B` 1.0 :`A` 1.0) 0.0)
  (`KismetSystemLibrary.PrintString` (`KismetStringLibrary.Concat_StrStr` "Attacking : " (`KismetStringLibrary.Conv_BoolToString` (`.IsAttacking` (`self.GetAllInputValue`)))) true true (struct :`G` 0.66 :`B` 1.0 :`A` 1.0) 0.0)
  (`KismetSystemLibrary.PrintString` (`KismetStringLibrary.Concat_StrStr` "Camera : " (`KismetStringLibrary.Conv_Vector2dToString` (`.Look 2D Axis` (`self.GetAllInputValue`)))) true true (struct :`G` 0.66 :`B` 1.0 :`A` 1.0) 0.0)
  (`KismetSystemLibrary.PrintString` (`KismetStringLibrary.Concat_StrStr` "Movement : " (`KismetStringLibrary.Conv_Vector2dToString` (`self.GetAllInputValue`))) true true (struct :`G` 0.66 :`B` 1.0 :`A` 1.0) 0.0)
  (set `self.Sprinting` (> (`KismetMathLibrary.VSize` (`self.GetVelocity`)) 10.0)))

(event `EnhancedInput|/Game/CFTUD/Blueprints/Player/Input/IA_Attack`
  (params (ActionValue :type Boolean) (ElapsedSeconds :type "Float (single-precision)") (TriggeredSeconds :type "Float (single-precision)"))
  (:`Started`
    (`|PlayMontage` (`self.Mesh`) (`self.Attack Anim`))))

(event `EnhancedInput|/Game/CFTUD/Blueprints/Player/Input/IA_Block`
  (params (ActionValue :type Boolean) (ElapsedSeconds :type "Float (single-precision)") (TriggeredSeconds :type "Float (single-precision)"))
  (:`Started`
    (`|PlayMontage` (`self.Mesh`) (`self.Block Anim`))))

(event `EnhancedInput|/Game/CFTUD/Blueprints/Player/Input/IA_Dodge`
  (params (ActionValue :type Boolean) (ElapsedSeconds :type "Float (single-precision)") (TriggeredSeconds :type "Float (single-precision)"))
  (:`Started`
    (`|PlayMontage` (`self.Mesh`) (`self.Dodge Anim`))))

(event `EnhancedInput|/Game/CFTUD/Blueprints/Player/Input/IA_Interract`
  (params (ActionValue :type Boolean) (ElapsedSeconds :type "Float (single-precision)") (TriggeredSeconds :type "Float (single-precision)"))
  (:`Started`
    (`|PlayMontage` (`self.Mesh`) (`self.Interract Anim`))))

(event `EnhancedInput|/Game/CFTUD/Blueprints/Player/Input/IA_SwitchCombatExplorationMode`
  (params (ActionValue :type Boolean) (ElapsedSeconds :type "Float (single-precision)") (TriggeredSeconds :type "Float (single-precision)"))
  (:`Started`
    (if (`self.PlayingMode`)
      (set `self.PlayingMode` false)
      (else
        (set `self.PlayingMode` true)))))

(event `EnhancedInput|/Game/CFTUD/Blueprints/Player/Input/IA_Sprint`
  (params (ActionValue :type Boolean) (ElapsedSeconds :type "Float (single-precision)") (TriggeredSeconds :type "Float (single-precision)"))
  (:`Started`
    (if (`self.Sprinting`)
      (set `self.Sprinting` false)
      (else
        (set `self.Sprinting` true)))))

(fn `GetAllInputValue`
  (returns (`Movement 2D Axis` :type "Vector2D Structure") (`Look 2D Axis` :type "Vector2D Structure") (IsAttacking :type Boolean) (IsBlocking :type Boolean) (IsDodging :type Boolean) (IsInteracting :type Boolean) (PlayingMode :type String) (IsSprinting :type Boolean) (IsJumping :type Boolean))
  (return (`|GetInputActionValue`) (`|GetInputActionValue`) (`|GetInputActionValue`) (`|GetInputActionValue`) (`|GetInputActionValue`) (`|GetInputActionValue`) (`KismetMathLibrary.SelectString` "Combat" "Exploration" (`self.PlayingMode`)) (`self.Sprinting`) (`|GetInputActionValue`)))

(fn `UserConstructionScript`)