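; Player character child Blueprint handling melee attacks, dodging and a spectral special attack.
; IA_Attack plays a kick bash in FightMode, otherwise advances a looping three-slash montage combo through the Selection enum.
; Dodge spends stamina, pauses regeneration and disables input, while the block input is unwired.
; BeginPlay caches the Spectral, Ruined and Corrupted stones; the special attack activates an effect when SpectralStone's selected spell is Spectral.
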(event `EnhancedInput|/Game/CFTUD/Blueprints/Player/Input/IMC_SpecialAttack`
  (params (ActionValue :type Boolean) (ElapsedSeconds :type "Float (single-precision)") (TriggeredSeconds :type "Float (single-precision)"))
  (:`Triggered`
    (switch `/Game/CFTUD/Blueprints/Player/Enum/SpellEnum` (`/Game/CFTUD/Blueprints/Object/BP_SpectralStone.Spell Selection` (`self.SpectralStone`))
      (:`NewEnumerator0`
        (`KismetSystemLibrary.PrintString` "SpectrallAttaque" true true (struct :`R` 1.0 :`G` 0.083818 :`A` 1.0))
        (`ActorComponent.Activate` (`self.SpectralEffect`) false)
        (`KismetSystemLibrary.PrintString` "Power")))))

(event `EnhancedInput|/Game/CFTUD/Blueprints/Player/Input/IA_Attack`
  (params (ActionValue :type Boolean) (ElapsedSeconds :type "Float (single-precision)") (TriggeredSeconds :type "Float (single-precision)"))
  (bind _returnvalue (`GameplayStatics.GetPlayerController` 0))
  (bind _selection (`self.Selection`))
  (bind _returnvalue_2 (`|GetEnumeratorNameAsString` _selection))
  ;[1 1 1] Attaque
  (:`Triggered`
    (if (and (not (`self.Attack?`)) (`self.FightMode`))
      (`KismetSystemLibrary.PrintString` "Block")
      (set `self.Attack?` true)
      (`self.DisableInput` _returnvalue)
      (`|PlayMontage` (`self.Mesh`) "/Game/CFTUD/Characters/AnimTest/Combat/AM_KickBash.AM_KickBash"
        (:`OnCompleted`
          (`self.EnableInput` _returnvalue)
          (set `self.Attack?` false)
          (`KismetSystemLibrary.PrintString` "Hello")
          (set `self.forward` 0.0)
          (set `self.right` 0.0)))
      (elif (not (`self.Attack?`))
        (set `self.CanDodge` false)
        (`KismetSystemLibrary.PrintString` "Attaque !!!!!!!!!!!!!!!!!!!!!!!!!!!!!!!!!!!!!!!!!!!!!!!!!!!!!!!!!")
        (switch `/Game/CFTUD/Blueprints/Player/Enum/AttackEnum` _selection
          (:`NewEnumerator0`
            (set `self.Attack?` true)
            (`KismetSystemLibrary.PrintString` _returnvalue_2 true true (struct :`G` 0.66 :`B` 1.0 :`A` 1.0) 0.0)
            (`|PlayMontage` (`self.Mesh`) "/Game/Import/AnimKnightMixamo/SwordSlash1.SwordSlash1"
              (:`then`
                (bind _output_get (set `self.Selection` "NewEnumerator1"))
                (`KismetSystemLibrary.PrintString` (`|GetEnumeratorNameAsString` _output_get) true true (struct :`G` 0.66 :`B` 1.0 :`A` 1.0) 0.0))
              (:`OnCompleted`
                (set `self.CanDodge` true)
                (set `self.Attack?` false :!label _label))
              (:`OnInterrupted`
                (goto _label))))
          (:`NewEnumerator1`
            (set `self.Attack?` true)
            (`KismetSystemLibrary.PrintString` _returnvalue_2 true true (struct :`G` 0.66 :`B` 1.0 :`A` 1.0) 0.0)
            (`|PlayMontage` (`self.Mesh`) "/Game/Import/AnimKnightMixamo/AttackSlash2.AttackSlash2"
              (:`then`
                (bind _output_get_2 (set `self.Selection` "NewEnumerator2"))
                (`KismetSystemLibrary.PrintString` (`|GetEnumeratorNameAsString` _output_get_2) true true (struct :`G` 0.66 :`B` 1.0 :`A` 1.0) 0.0))
              (:`OnCompleted`
                (set `self.CanDodge` true)
                (set `self.Attack?` false :!label _label_2))
              (:`OnInterrupted`
                (goto _label_2))))
          (:`NewEnumerator2`
            (set `self.Attack?` true)
            (`KismetSystemLibrary.PrintString` _returnvalue_2 true true (struct :`G` 0.66 :`B` 1.0 :`A` 1.0) 0.0)
            (`|PlayMontage` (`self.Mesh`) "/Game/CFTUD/Characters/AnimTest/Combat/AM_Slash3.AM_Slash3"
              (:`then`
                (bind _output_get_3 (set `self.Selection` "NewEnumerator0"))
                (`KismetSystemLibrary.PrintString` (`|GetEnumeratorNameAsString` _output_get_3) true true (struct :`G` 0.66 :`B` 1.0 :`A` 1.0) 0.0))
              (:`OnCompleted`
                (set `self.CanDodge` true)
                (set `self.Attack?` false :!label _label_3))
              (:`OnInterrupted`
                (goto _label_3)))))))))

(event `EnhancedInput|/Game/CFTUD/Blueprints/Player/Input/IA_Dodge`
  (params (ActionValue :type Boolean) (ElapsedSeconds :type "Float (single-precision)") (TriggeredSeconds :type "Float (single-precision)"))
  (:`Triggered`
    (if (and (`self.CanDodge`) (> (`self.Stamina`) 20.0) (not (`NavMovementComponent.IsFalling` (`self.CharacterMovement`))))
      (set `self.dodge` true)
      (set `self.forward` 0.0)
      (set `self.right` 0.0)
      (set `self.Stamina` (- (`self.Stamina`) 20.0))
      (`KismetSystemLibrary.K2_PauseTimerHandle` (`self.TimerHandleRegenStamina`))
      (`self.DisableInput` (`GameplayStatics.GetPlayerController` 0)))))

(event `EnhancedInput|/Game/CFTUD/Blueprints/Player/Input/IA_Block`
  (params (ActionValue :type Boolean) (ElapsedSeconds :type "Float (single-precision)") (TriggeredSeconds :type "Float (single-precision)")))

(event `self.ReceiveBeginPlay`
  (`parent.ReceiveBeginPlay`)
  (bind _returnvalue (`GameplayStatics.GetActorOfClass` "/Game/CFTUD/Blueprints/Object/BP_SpectralStone.BP_SpectralStone_C"))
  (set `self.SpectralStone` _returnvalue)
  (bind _returnvalue_2 (`GameplayStatics.GetActorOfClass` "/Game/CFTUD/Blueprints/Object/BP_RuinedStone.BP_RuinedStone_C"))
  (set `self.RuinedStone` _returnvalue_2)
  (bind _returnvalue_3 (`GameplayStatics.GetActorOfClass` "/Game/CFTUD/Blueprints/Object/BP_CorruptedStone.BP_CorruptedStone_C"))
  (set `self.corrupted` _returnvalue_3))

(event `self.ReceiveTick`
  (params (DeltaSeconds :type "Float (single-precision)"))
  (`parent.ReceiveTick` DeltaSeconds))

(fn `UserConstructionScript`
  (`parent.UserConstructionScript`))