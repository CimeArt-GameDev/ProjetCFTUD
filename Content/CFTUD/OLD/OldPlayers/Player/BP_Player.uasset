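; BP_Player is a player Blueprint, kept in an OLD folder, that plays attack, block and dodge montages from Enhanced Input actions.
; BeginPlay adds the player mapping context, and any key press records whether a keyboard is used.
; Tick prints input state gathered by GetAllInputValue and derives Sprinting from velocity above a small threshold.
; Interact and jump report false, while sprint toggle, mode toggle and interact montage logic are disconnected.
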(event `Key|AnyKey`
  (params (Key :type "Key Structure"))
  (:`Pressed`
    (set `self.IsKeyboardUsed` (`KismetInputLibrary.Key_IsKeyboardKey` Key))))

(event `self.ReceiveBeginPlay`
  (`EnhancedInputSubsystemInterface.AddMappingContext` (pcsubsystem `EnhancedInputLocalPlayerSubsystem` (`GameplayStatics.GetPlayerController` 0)) "/Game/CFTUD/OLD/OldPlayers/Player/Input/IMC_Player.IMC_Player" 0 (struct)))

(event `self.ReceiveTick`
  (params (DeltaSeconds :type "Float (single-precision)"))
  (`KismetSystemLibrary.PrintString` (`KismetStringLibrary.Concat_StrStr` "Jumping : " (`KismetStringLibrary.Conv_BoolToString` (`.IsJumping` (`self.GetAllInputValue`)))) true true (struct :`G` 0.66 :`B` 1.0 :`A` 1.0) 0.0)
  (`KismetSystemLibrary.PrintString` (`KismetStringLibrary.Concat_StrStr` "Sprinting : " (`KismetStringLibrary.Conv_BoolToString` (`.IsSprinting` (`self.GetAllInputValue`)))) true true (struct :`G` 0.66 :`B` 1.0 :`A` 1.0) 0.0)
  (`KismetSystemLibrary.PrintString` (`KismetStringLibrary.Concat_StrStr` "Playing Mode : " (`.PlayingMode` (`self.GetAllInputValue`))) true true (struct :`G` 0.66 :`B` 1.0 :`A` 1.0) 0.0)
  (`KismetSystemLibrary.PrintString` (`KismetStringLibrary.Concat_StrStr` "Interacting : " (`KismetStringLibrary.Conv_BoolToString` (`.IsInteracting` (`self.GetAllInputValue`)))) true true (struct :`G` 0.66 :`B` 1.0 :`A` 1.0) 0.0)
  (`KismetSystemLibrary.PrintString` (`KismetStringLibrary.Concat_StrStr` "Dodging : " (`KismetStringLibrary.Conv_BoolToString` (`.IsDodging` (`self.GetAllInputValue`)))) true true (struct :`G` 0.66 :`B` 1.0 :`A` 1.0) 0.0)
  (`KismetSystemLibrary.PrintString` (`KismetStringLibrary.Concat_StrStr` "Blocking : " (`KismetStringLibrary.Conv_BoolToString` (`.IsBlocking` (`self.GetAllInputValue`)))) true true (struct :`G` 0.66 :`B` 1.0 :`A` 1.0) 0.0)
  (`KismetSystemLibrary.PrintString` (`KismetStringLibrary.Concat_StrStr` "Attacking : " (`KismetStringLibrary.Conv_BoolToString` (`.IsAttacking` (`self.GetAllInputValue`)))) true true (struct :`G` 0.66 :`B` 1.0 :`A` 1.0) 0.0)
  (`KismetSystemLibrary.PrintString` (`KismetStringLibrary.Concat_StrStr` "Camera : " (`KismetStringLibrary.Conv_Vector2dToString` (`.Look 2D Axis` (`self.GetAllInputValue`)))) true true (struct :`G` 0.66 :`B` 1.0 :`A` 1.0) 0.0)
  (`KismetSystemLibrary.PrintString` (`KismetStringLibrary.Concat_StrStr` "Movement : " (`KismetStringLibrary.Conv_Vector2dToString` (`self.GetAllInputValue`))) true true (struct :`G` 0.66 :`B` 1.0 :`A` 1.0) 0.0)
  (set `self.Sprinting` (> (`KismetMathLibrary.VSize` (`self.GetVelocity`)) 10.0)))

(event `EnhancedInput|/Game/CFTUD/OLD/OldPlayers/Player/Input/IA_Attack`
  (params (ActionValue :type Boolean) (ElapsedSeconds :type "Float (double-precision)") (TriggeredSeconds :type "Float (double-precision)") (InputAction :type "InputAction Object Reference" :default "/Game/CFTUD/OLD/OldPlayers/Player/Input/IA_Attack.IA_Attack"))
  (:`Started`
    (`|PlayMontage` (`self.Mesh`) (`self.Attack Anim`))))

(event `EnhancedInput|/Game/CFTUD/OLD/OldPlayers/Player/Input/IA_Block`
  (params (ActionValue :type Boolean) (ElapsedSeconds :type "Float (double-precision)") (TriggeredSeconds :type "Float (double-precision)") (InputAction :type "InputAction Object Reference" :default "/Game/CFTUD/OLD/OldPlayers/Player/Input/IA_Block.IA_Block"))
  (:`Started`
    (`|PlayMontage` (`self.Mesh`) (`self.Block Anim`))))

(event `EnhancedInput|/Game/CFTUD/OLD/OldPlayers/Player/Input/IA_Dodge`
  (params (ActionValue :type Boolean) (ElapsedSeconds :type "Float (double-precision)") (TriggeredSeconds :type "Float (double-precision)") (InputAction :type "InputAction Object Reference" :default "/Game/CFTUD/OLD/OldPlayers/Player/Input/IA_Dodge.IA_Dodge"))
  (:`Started`
    (`|PlayMontage` (`self.Mesh`) (`self.Dodge Anim`))))

(fn `GetAllInputValue`
  (returns (`Movement 2D Axis` :type "Vector2D Structure") (`Look 2D Axis` :type "Vector2D Structure") (IsAttacking :type Boolean) (IsBlocking :type Boolean) (IsDodging :type Boolean) (IsInteracting :type Boolean) (PlayingMode :type String) (IsSprinting :type Boolean) (IsJumping :type Boolean))
  (return (`|GetInputActionValue`) (`|GetInputActionValue`) (`|GetInputActionValue`) (`|GetInputActionValue`) (`|GetInputActionValue`) false (`KismetMathLibrary.SelectString` "Combat" "Exploration" (`self.PlayingMode`)) (`self.Sprinting`) false))

(fn `UserConstructionScript`)