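; Player character child Blueprint, apparently a test version, adding melee attacks and a stamina-costed dodge.
; The attack input plays a kick-bash in FightMode, otherwise cycles a three-slash montage combo via Selection, advanced as each montage starts.
; Dodge spends stamina, pauses its regen timer and disables input while flags gate overlapping actions.
; BeginPlay caches three stone actors, used only by disconnected spell code; construction attaches Niagara to a thigh socket.
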(event `EnhancedInput|/Game/CFTUD/OLD/OldPlayers/Player/Input/IA_Attack`
  (params (ActionValue :type Boolean) (ElapsedSeconds :type "Float (double-precision)") (TriggeredSeconds :type "Float (double-precision)") (InputAction :type "InputAction Object Reference" :default "/Game/CFTUD/OLD/OldPlayers/Player/Input/IA_Attack.IA_Attack"))
  (bind _returnvalue (`GameplayStatics.GetPlayerController` 0))
  (bind _selection (`self.Selection`))
  (bind _returnvalue_2 (`|GetEnumeratorNameAsString` _selection))
  ;[1 1 1] Attaque
  (:`Started`
    (if (and (not (`self.Attack?`)) (`self.FightMode`))
      (`KismetSystemLibrary.PrintString` "Block")
      (set `self.Attack?` true)
      (`self.DisableInput` _returnvalue)
      (`|PlayMontage` (`self.Mesh`) "/Game/CFTUD/OLD/OldPlayers/Animations/AnimPlayer/AM_KickBash_Retargeted1.AM_KickBash_Retargeted1"
        (:`OnCompleted`
          (`self.EnableInput` _returnvalue)
          (set `self.Attack?` false)
          (`KismetSystemLibrary.PrintString` "Hello")
          (set `self.forward` 0.0)
          (set `self.right` 0.0)))
      (elif (not (`self.Attack?`))
        (set `self.CanDodge` false)
        (`KismetSystemLibrary.PrintString` "Attaque !!!!!!!!!!!!!!!!!!!!!!!!!!!!!!!!!!!!!!!!!!!!!!!!!!!!!!!!!")
        (switch `/Game/CFTUD/OLD/OldPlayers/Player/Enum/AttackEnum` _selection
          (:`NewEnumerator0`
            (set `self.Attack?` true)
            (`KismetSystemLibrary.PrintString` _returnvalue_2 true true (struct :`G` 0.66 :`B` 1.0 :`A` 1.0) 0.0)
            (`|PlayMontage` (`self.Mesh`) "/Game/CFTUD/OLD/OldPlayers/Animations/AnimNewMannequin/SwordSlash1_Retargeted.SwordSlash1_Retargeted"
              (:`then`
                (bind _output_get (set `self.Selection` "NewEnumerator1"))
                (`KismetSystemLibrary.PrintString` (`|GetEnumeratorNameAsString` _output_get) true true (struct :`G` 0.66 :`B` 1.0 :`A` 1.0) 0.0))
              (:`OnCompleted`
                (set `self.CanDodge` true)
                (set `self.Attack?` false :!label _label))
              (:`OnInterrupted`
                (goto _label))))
          (:`NewEnumerator1`
            (set `self.Attack?` true)
            (`KismetSystemLibrary.PrintString` _returnvalue_2 true true (struct :`G` 0.66 :`B` 1.0 :`A` 1.0) 0.0)
            (`|PlayMontage` (`self.Mesh`) "/Game/CFTUD/OLD/OldPlayers/Animations/AnimNewMannequin/AttackSlash2_Retargeted.AttackSlash2_Retargeted"
              (:`then`
                (bind _output_get_2 (set `self.Selection` "NewEnumerator2"))
                (`KismetSystemLibrary.PrintString` (`|GetEnumeratorNameAsString` _output_get_2) true true (struct :`G` 0.66 :`B` 1.0 :`A` 1.0) 0.0))
              (:`OnCompleted`
                (set `self.CanDodge` true)
                (set `self.Attack?` false :!label _label_2))
              (:`OnInterrupted`
                (goto _label_2))))
          (:`NewEnumerator2`
            (set `self.Attack?` true)
            (`KismetSystemLibrary.PrintString` _returnvalue_2 true true (struct :`G` 0.66 :`B` 1.0 :`A` 1.0) 0.0)
            (`|PlayMontage` (`self.Mesh`) "/Game/CFTUD/OLD/OldPlayers/Animations/AnimNewMannequin/AM_Slash3_Retargeted.AM_Slash3_Retargeted"
              (:`then`
                (bind _output_get_3 (set `self.Selection` "NewEnumerator0"))
                (`KismetSystemLibrary.PrintString` (`|GetEnumeratorNameAsString` _output_get_3) true true (struct :`G` 0.66 :`B` 1.0 :`A` 1.0) 0.0))
              (:`OnCompleted`
                (set `self.CanDodge` true)
                (set `self.Attack?` false :!label _label_3))
              (:`OnInterrupted`
                (goto _label_3)))))))))

(event `EnhancedInput|/Game/CFTUD/OLD/OldPlayers/Player/Input/IA_Dodge`
  (params (ActionValue :type Boolean) (ElapsedSeconds :type "Float (double-precision)") (TriggeredSeconds :type "Float (double-precision)") (InputAction :type "InputAction Object Reference" :default "/Game/CFTUD/OLD/OldPlayers/Player/Input/IA_Dodge.IA_Dodge"))
  (:`Triggered`
    (if (and (`self.CanDodge`) (> (`self.Stamina`) 20.0) (not (`NavMovementComponent.IsFalling` (`self.CharacterMovement`))))
      (set `self.dodge` true)
      (set `self.forward` 0.0)
      (set `self.right` 0.0)
      (set `self.Stamina` (- (`self.Stamina`) 20.0))
      (`KismetSystemLibrary.K2_PauseTimerHandle` (`self.TimerHandleRegenStamina`))
      (`self.DisableInput` (`GameplayStatics.GetPlayerController` 0))))
  (:`Completed`
    (set `self.dodge` false)))

(event `EnhancedInput|/Game/CFTUD/OLD/OldPlayers/Player/Input/IA_Block`
  (params (ActionValue :type Boolean) (ElapsedSeconds :type "Float (double-precision)") (TriggeredSeconds :type "Float (double-precision)") (InputAction :type "InputAction Object Reference" :default "/Game/CFTUD/OLD/OldPlayers/Player/Input/IA_Block.IA_Block")))

(event `self.ReceiveBeginPlay`
  (`parent.ReceiveBeginPlay`)
  (bind _returnvalue (`GameplayStatics.GetActorOfClass` "/Game/CFTUD/Blueprints/Object/BP_SpectralStone.BP_SpectralStone_C"))
  (set `self.SpectralStone` _returnvalue)
  (bind _returnvalue_2 (`GameplayStatics.GetActorOfClass` "/Game/CFTUD/Blueprints/Object/BP_RuinedStone.BP_RuinedStone_C"))
  (set `self.RuinedStone` _returnvalue_2)
  (bind _returnvalue_3 (`GameplayStatics.GetActorOfClass` "/Game/CFTUD/Blueprints/Object/BP_CorruptedStone.BP_CorruptedStone_C"))
  (set `self.corrupted` _returnvalue_3))

(event `self.ReceiveTick`
  (params (DeltaSeconds :type "Float (single-precision)"))
  (`parent.ReceiveTick` DeltaSeconds))

(fn `UserConstructionScript`
  (`parent.UserConstructionScript`)
  (`SceneComponent.K2_AttachToComponent` (`self.Niagara`) (`self.Mesh`) "thigh_lSocket" "KeepWorld" "KeepWorld" "KeepWorld" true))