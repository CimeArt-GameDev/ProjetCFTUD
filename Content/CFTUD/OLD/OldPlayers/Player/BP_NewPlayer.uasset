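; BP_NewPlayer is a player pawn Blueprint that handles Enhanced Input for movement and camera look.
; Look input turns the controller at a frame-time-scaled rate, while move input is stored as Forward and Right values.
; AdjustCameraAngle adds automatic yaw from sideways input, shaped by an exponent and scaled by horizontal speed, though nothing here calls it.
; Tick stores a Direction from CalculateDirection, whose camera-versus-capsule rotation math is left unconnected.
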(event `self.ReceiveBeginPlay`
  (`EnhancedInputSubsystemInterface.AddMappingContext` (pcsubsystem `EnhancedInputLocalPlayerSubsystem` (`GameplayStatics.GetPlayerController` 0)) "/Game/CFTUD/OLD/OldPlayers/Player/Input/IMC_Player.IMC_Player" 0 (struct)))

(event `EnhancedInput|/Game/CFTUD/OLD/OldPlayers/Player/Input/IA_Look`
  (params (ActionValue :type "Vector2D Structure") (ElapsedSeconds :type "Float (double-precision)") (TriggeredSeconds :type "Float (double-precision)") (InputAction :type "InputAction Object Reference" :default "/Game/CFTUD/OLD/OldPlayers/Player/Input/IA_Look.IA_Look"))
  (:`Triggered`
    (`self.AddControllerYawInput` (* ActionValue_X (`self.CameraRotationRate`) (`GameplayStatics.GetWorldDeltaSeconds`)))
    (`self.AddControllerPitchInput` (* ActionValue_Y (`self.CameraRotationRate`) (`GameplayStatics.GetWorldDeltaSeconds`)))))

(event `AdjustCameraAngle`
  (bind (_returnvalue_x _returnvalue_y) (`KismetMathLibrary.BreakVector` (`self.GetVelocity`)))
  (bind _yinput (`self.yInput`))
  (bind (_returnvalue_x_2 _returnvalue_y_2) (`KismetMathLibrary.BreakVector` (`KismetMathLibrary.Normal` (`KismetMathLibrary.MakeVector` (`self.GetInputAxisValue`) (`self.GetInputAxisValue`)))))
  (bind _output_get (set `self.yInput` _returnvalue_y_2))
  (if (!= _output_get 0.0)
    (`self.AddControllerYawInput` (* (* _yinput (`KismetMathLibrary.MultiplyMultiply_FloatFloat` (`KismetMathLibrary.Abs` _yinput) (`self.camAngleExponent`))) 100.0 (/ (`KismetMathLibrary.VSize` (`KismetMathLibrary.MakeVector` _returnvalue_x _returnvalue_y)) 379.0) (`self.camRotationFactor`) (`GameplayStatics.GetWorldDeltaSeconds`)))))

(event `EnhancedInput|/Game/CFTUD/OLD/OldPlayers/Player/Input/IA_Move`
  (params (ActionValue :type "Vector2D Structure") (ElapsedSeconds :type "Float (double-precision)") (TriggeredSeconds :type "Float (double-precision)") (InputAction :type "InputAction Object Reference" :default "/Game/CFTUD/OLD/OldPlayers/Player/Input/IA_Move.IA_Move"))
  (:`Triggered`
    (set `self.forward` ActionValue_X :!label _label)
    (set `self.right` ActionValue_Y))
  (:`Completed`
    (goto _label)))

(event `self.ReceiveTick`
  (params (DeltaSeconds :type "Float (single-precision)"))
  (bind (_returnvalue_x _returnvalue_y) (`KismetMathLibrary.BreakVector2D` (`|GetInputActionValue`)))
  (set `self.direction` (`self.CalculateDirection` (`self.Camera`) (`self.CapsuleComponent`) _returnvalue_x _returnvalue_y)))

(fn `UserConstructionScript`)